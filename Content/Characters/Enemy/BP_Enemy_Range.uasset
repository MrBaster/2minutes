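; BP_Enemy_Range is a ranged enemy that periodically fires projectiles, built on a parent enemy Blueprint.
; On BeginPlay it runs the parent logic, halves its inherited SpeedBoost stat and starts a looping fire timer with a randomized initial delay.
; Each timer tick spawns a RangeEnemyBullet at the enemy's location, oriented along the MyMovePoint vector and carrying its Damage stat, and prints a debug message.
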(event `self.ReceiveBeginPlay`
  (bind (_hp _damage _speedboost _hpreward) (break `/Game/Characters/Enemy/EnemyStats` (`self.Stats`)))
  (`parent.ReceiveBeginPlay`)
  (set `self.Stats` (make `/Game/Characters/Enemy/EnemyStats` _hp _damage (/ _speedboost 2.0) _hpreward))
  (`KismetSystemLibrary.K2_SetTimerDelegate` (delegate `Range_Fire`) 6.0 true 0.0 1.0))

(event `Range_Fire`
  (bind (_stats_hp _stats_damage) (break `/Game/Characters/Enemy/EnemyStats` (`self.Stats`)))
  (`KismetSystemLibrary.PrintString` "Fire" true true (struct :`R` 1.0 :`G` 0.009182 :`A` 1.0) 4.0)
  (`|SpawnActorFromClass` "/Game/ThirdPerson/Blueprints/Bullet/RangeEnemyBullet.RangeEnemyBullet_C" (`KismetMathLibrary.MakeTransform` (`self.K2_GetActorLocation`) (`KismetMathLibrary.Conv_VectorToRotator` (`self.MyMovePoint`))) "AlwaysSpawn" "MultiplyWithRoot" null _stats_damage null))

(fn `UserConstructionScript`
  (`parent.UserConstructionScript`))