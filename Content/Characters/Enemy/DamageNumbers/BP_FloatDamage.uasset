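; BP_FloatDamage is an actor that shows a floating damage number in the world, then removes itself.
; On BeginPlay it casts its Damage widget component to W_FloatDamage and passes in DamageVal and the IsCrit flag.
; A Timeline then nudges the actor upward each update by an alpha-scaled offset added to its current height, and destroys it when finished.
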(event `self.ReceiveBeginPlay`
  (bind (_returnvalue_x _returnvalue_y _returnvalue_z) (`KismetMathLibrary.BreakVector` (`self.K2_GetActorLocation` self)))
  (bind _asw_float_damage (cast `/Game/Characters/Enemy/DamageNumbers/W_FloatDamage` (`WidgetComponent.GetUserWidgetObject` (`self.Damage`))))
  (`/Game/Characters/Enemy/DamageNumbers/W_FloatDamage.SetDamage` _asw_float_damage (`self.DamageVal`) (`self.IsCrit`))
  (bind (_direction _alpha) (`Timeline|Timeline`)
    (:`Update`
      (`self.K2_SetActorLocation` self (`KismetMathLibrary.MakeVector` _returnvalue_x _returnvalue_y (+ _returnvalue_z (`KismetMathLibrary.Lerp` 0.0 2.0 _alpha))) false false))
    (:`Finished`
      (`self.K2_DestroyActor`))))

(fn `UserConstructionScript`)