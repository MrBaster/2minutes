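; Troll enemy with a flipbook sprite, extending a parent enemy with its own stats and a recurring area attack.
; A self-rearming timer fires BigHit, which halts movement, plays the attack flipbook and waits a frame-rate-derived delay.
; It then spawns a radius-matched Niagara effect, deals crit-type radial damage around Sphere1 and resumes walking.
; When destroyed, it spawns a Troll_Dead actor in its place.
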(event `self.ReceiveDestroyed`
  (`|SpawnActorFromClass` "/Game/Characters/Cringe/Troll_Dead.Troll_Dead_C" (`KismetMathLibrary.MakeTransform` (`self.K2_GetActorLocation`) (`SceneComponent.K2_GetComponentRotation` (`self.RunFB`)) (`SceneComponent.K2_GetComponentScale` (`self.RunFB`))) "Undefined" "MultiplyWithRoot" null null))

(event `self.ReceiveBeginPlay`
  (set `self.Stats` (make `/Game/Characters/Enemy/EnemyStats` 10000.0 100.0 1.0 5.0))
  (`parent.ReceiveBeginPlay`)
  (bind _returnvalue (`KismetSystemLibrary.K2_SetTimerDelegate` (delegate `BigHit`) 3.0 :!label _label))
  (set `self.BigHitTimer` _returnvalue))

(event `BigHit`
  (bind _sphere1 (`self.Sphere1`))
  (bind _runfb (`self.RunFB`))
  (bind _sphere1_2 (`self.Sphere1`))
  (`KismetSystemLibrary.K2_PauseTimerHandle` (`self.BigHitTimer`))
  (set `self.CanIMove` false)
  (`PaperFlipbookComponent.SetFlipbook` _runfb "/Game/Characters/Sprites/Troll/Sprites/Attack/Troll_01_1_ATTACK.Troll_01_1_ATTACK")
  (`KismetSystemLibrary.Delay` (* (/ 1.0 (`PaperFlipbookComponent.GetFlipbookFramerate` _runfb)) 7.0))
  ;[1 1 1] Attack VFX
  (bind _returnvalue (`NiagaraFunctionLibrary.SpawnSystemAtLocation` "/Game/VFX/Systems/PS_TrollAttack_01.PS_TrollAttack_01" (`SceneComponent.K2_GetComponentLocation` _sphere1_2) (struct) (1.0 1.0 1.0) true false "AutoRelease"))
  (`NiagaraComponent.SetVariableFloat` _returnvalue "Radius" (`SphereComponent.SphereRadius` _sphere1_2))
  (`ActorComponent.ToggleActive` _returnvalue)
  (`GameplayStatics.ApplyRadialDamage` :`BaseDamage` 100.0 :`Origin` (`SceneComponent.K2_GetComponentLocation` _sphere1) :`DamageRadius` (`SphereComponent.SphereRadius` _sphere1) :`DamageTypeClass` "/Game/ThirdPerson/Blueprints/Bullet/DT_Crit.DT_Crit_C" :`DamageCauser` self :`InstigatedByController` null :`bDoFullDamage` true :`DamagePreventionChannel` "ECC_Pawn")
  (`KismetSystemLibrary.K2_UnPauseTimerHandle` (`self.BigHitTimer`))
  (set `self.CanIMove` true)
  (`PaperFlipbookComponent.SetFlipbook` (`self.RunFB`) "/Game/Characters/Sprites/Troll/Sprites/Walk/Troll_01_1_WALK.Troll_01_1_WALK")
  (goto _label))

(fn `UserConstructionScript`
  (`parent.UserConstructionScript`))