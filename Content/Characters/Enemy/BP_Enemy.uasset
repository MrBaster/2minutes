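; Enemy character that launches itself at the player, deals damage and dies on contact, with starting HP scaled by DeltaTimeSum.
; Looping timers drive movement through repeated LaunchCharacter calls and clamp the resulting velocity.
; Damage spawns floating numbers, applies knockback scaled by a player stat and recolours the sphere from green to red as HP falls.
; Death spawns an explosion and one weighted-random drop carrying the XP reward.
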(event `self.ReceiveBeginPlay`
  (bind _stats_hp (break `/Game/Characters/Enemy/EnemyStats` (`self.Stats`)))
  (bind _output_get (set `self.HPMax` (+ _stats_hp (* (`self.DeltaTimeSum`) 0.4))))
  (set `self.HPCurrent` _output_get)
  (`self.UpdateHPVFX`)
  (`KismetSystemLibrary.K2_SetTimerDelegate` (delegate `Move`) 0.1 true)
  (`KismetSystemLibrary.K2_SetTimerDelegate` (delegate `ClampVelocity`) 0.07 true))

(event `ClampVelocity`
  (bind _returnvalue (+ 350.0 0.0))
  (`self.LaunchCharacter` (`KismetMathLibrary.ClampVectorSize` (`CharacterMovementComponent.GetLastUpdateVelocity` (`self.CharacterMovement`)) (* _returnvalue -1.0) _returnvalue) true true))

(event `Move`
  (bind (_returnvalue_x _returnvalue_y) (`KismetMathLibrary.BreakVector` (`self.GetMovementPoint` false)))
  (`self.LaunchCharacter` (* (`self.GetMovementPoint` false) 700 (`self.GetSpeedBoost`)))
  (`SceneComponent.K2_SetRelativeRotation` (`self.RunFB`) (`KismetMathLibrary.MakeRotator` 0.0 0.0 (`KismetMathLibrary.SelectFloat` 90.0 -90.0 (> _returnvalue_y 0.0))) false false))

(event `self.ReceiveTick`
  (params (DeltaSeconds :type "Float (single-precision)")))

(event `self.ReceiveAnyDamage`
  (params (Damage :type "Float (single-precision)") (DamageType :type "DamageType Object Reference") (InstigatedBy :type "Controller Object Reference") (DamageCauser :type "Actor Object Reference"))
  (bind (_stat_name _stat_value) (break `/Game/ThirdPerson/Blueprints/StatStructure` (`/Game/ThirdPerson/Blueprints/BP_ThirdPersonCharacter.GetStat` (`/Game/ThirdPerson/Blueprints/GetPlayerFuncLib.GetPlayer`) "NewEnumerator16")))
  (`self.SpawnFloatDamage` Damage (== (`GameplayStatics.GetObjectClass` DamageType) "/Game/ThirdPerson/Blueprints/Bullet/DT_Crit.DT_Crit_C"))
  (`self.Knockback` _stat_value)
  (bind _output_get (set `self.HPCurrent` (- (`self.HPCurrent`) Damage)))
  (`self.UpdateHPVFX`)
  (if (<= _output_get 0.0)
    (`self.Death` :!label _label)))

(event `self.CapsuleComponent.OnComponentHit`
  (params (HitComponent :type "PrimitiveComponent Object Reference") (OtherActor :type "Actor Object Reference") (OtherComp :type "PrimitiveComponent Object Reference") (NormalImpulse :type "Vector Structure") (Hit :type "HitResult Structure (by ref)"))
  (bind (_stats_hp _stats_damage) (break `/Game/Characters/Enemy/EnemyStats` (`self.Stats`)))
  (bind _asbp_third_person_character (cast `/Game/ThirdPerson/Blueprints/BP_ThirdPersonCharacter` OtherActor))
  (`GameplayStatics.ApplyDamage` _asbp_third_person_character _stats_damage)
  (goto _label))

(fn `Death`
  (`self.DropLoot`)
  (`GameplayStatics.SpawnEmitterAtLocation` "/Game/StarterContent/Particles/P_Explosion.P_Explosion" (`self.K2_GetActorLocation`))
  (`self.K2_DestroyActor`))

(fn `DropLoot`
  (locals (ChanceSum :type "Float (double-precision)") (CumulativeProbability :type "Float (double-precision)") (Rand :type "Float (double-precision)" :default 0.0))
  (bind (_stats_hp _stats_damage _stats_speedboost _stats_hpreward) (break `/Game/Characters/Enemy/EnemyStats` (`self.Stats`)))
  (bind _values (`BlueprintMapLibrary.Map_Values` (`self.DropChances`)))
  (for _array_element _values
    (set `local.ChanceSum` (+ _array_element (`local.ChanceSum`))))
  (set `local.Rand` (`KismetMathLibrary.RandomFloatInRange` 0.0 (`local.ChanceSum`)))
  (for (_array_element_2 _array_index) _values
    (set `local.CumulativeProbability` (+ _array_element_2 (`local.CumulativeProbability`)))
    (if (<= (`local.Rand`) (`local.CumulativeProbability`))
      (bind _keys (`BlueprintMapLibrary.Map_Keys` (`self.DropChances`)))
      (`|SpawnActorFromClass` (`|GetArrayItem` _keys _array_index) (`KismetMathLibrary.MakeTransform` (`self.K2_GetActorLocation`)) "Undefined" "MultiplyWithRoot" null _stats_hpreward null)
      (break))))

(fn `Knockback`
  (params (PowerMult :type "Float (double-precision)"))
  (`self.LaunchCharacter` (* (`self.GetMovementPoint` true) 900 PowerMult) true))

(fn `SpawnFloatDamage`
  (params (DamageVal :type "Float (double-precision)") (IsCrit :type Boolean))
  (bind (_returnvalue_x _returnvalue_y _returnvalue_z) (`KismetMathLibrary.BreakVector` (`self.K2_GetActorLocation` self)))
  (`|SpawnActorFromClass` "/Game/Characters/Enemy/DamageNumbers/BP_FloatDamage.BP_FloatDamage_C" (`KismetMathLibrary.MakeTransform` (`KismetMathLibrary.MakeVector` (+ _returnvalue_x (`KismetMathLibrary.RandomFloatInRange` -50.0 50.0)) (+ _returnvalue_y (`KismetMathLibrary.RandomFloatInRange` -50.0 50.0)) (+ _returnvalue_z 30.0))) "Undefined" "MultiplyWithRoot" null DamageVal IsCrit null))

(fn `UpdateHPVFX`
  (bind _returnvalue (`KismetMaterialLibrary.CreateDynamicMaterialInstance` "/Game/StarterContent/Materials/M_Tech_Hex_Tile_Pulse.M_Tech_Hex_Tile_Pulse"))
  (`MaterialInstanceDynamic.SetVectorParameterValue` _returnvalue "HPColour" (`KismetMathLibrary.LinearColorLerp` (struct :`R` 1.0 :`G` 0.015686 :`A` 1.0) (struct :`R` 0.031373 :`G` 1.0 :`A` 1.0) (/ (`self.HPCurrent`) (`self.HPMax`))))
  (`PrimitiveComponent.SetMaterial` (`self.Sphere`) 0 _returnvalue))

(fn `UserConstructionScript`)